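; Player-controlled F-18 aircraft driven by a JSBSim movement component, with mouse look and Tab toggling between third-person and cockpit cameras.
; Held keys set flags that Tick turns into per-frame steps of throttle (W/S), roll trim (A/D) and pitch trim (E/C).
; Values reach JSBSim engine or flight commands only on key press, not from Tick.
; BeginPlay caches the F-18C anim instance and enables input.
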(event EventBeginPlay
  (bind _asabp_west_fighter_f18c_showcase (Utilities|Casting|CastToABP_West_Fighter_F18C_Showcase (Components|SkeletalMesh|GetAnimInstance (Variables|Default|GetSkeletalMesh))))
  (Variables|Default|SetAs%20ABP%20West%20Fighter%20F18C%20Showcase _asabp_west_fighter_f18c_showcase)
  (Input|EnableInput 0))

(event EventTick
  (params (DeltaSeconds :type Float%20%28single-precision%29))
  (Utilities|FlowControl|Sequence
    (:then_0
      (if (Variables|Default|GetPressing%20S)
        (Math|Float|DecrementFloat (Variables|Default|GetThrottleValue))))
    (:then_1
      (if (Variables|Default|GetPressing%20W)
        (Math|Float|IncrementFloat (Variables|Default|GetThrottleValue))))
    (:then_2
      (if (Variables|Default|GetPressing%20A)
        (Variables|Default|SetRoll%20Trim (- (Variables|Default|GetRoll%20Trim) 0.01))))
    (:then_3
      (if (Variables|Default|GetPressing%20D)
        (Variables|Default|SetRoll%20Trim (+ (Variables|Default|GetRoll%20Trim) 0.01))))
    (:then_4
      (if (Variables|Default|GetPressing%20C)
        (Variables|Default|SetPitch%20Trim (- (Variables|Default|GetPitch%20Trim) 0.01))))
    (:then_5
      (if (Variables|Default|GetPressing%20E)
        (Variables|Default|SetPitch%20Trim (+ (Variables|Default|GetPitch%20Trim) 0.01))))))

(event Input|AxisEvents|InputAxisLookUp
  (params (AxisValue :type Float%20%28single-precision%29))
  ;[0.15 0.15 0.15 0.5] Camera
  (Pawn|Input|AddControllerPitchInput (* AxisValue -1.0)))

(event Input|AxisEvents|InputAxisLookRight
  (params (AxisValue :type Float%20%28single-precision%29))
  ;[0.15 0.15 0.15 0.5] Camera
  (Pawn|Input|AddControllerYawInput AxisValue))

(event Input|KeyboardEvents|W
  (params (Key :type Key%20Structure))
  (bind _jsbsimmovement (Variables|Default|GetJSBSimMovement))
  (bind _enginecommands (Variables|/Script/JSBSimFlightDynamicsModel.JSBSimMovementComponent|GetEngineCommands _jsbsimmovement))
  ;[1 1 1] 조종
  (:Pressed
    (Variables|Default|SetPressing%20W true)
    (for (_ _array_index) _enginecommands
      (Utilities|Struct|SetmembersinEngineCommand (Utilities|Array|Get(acopy) _enginecommands _array_index) (Variables|Default|GetThrottleValue))
      (Variables|/Script/JSBSimFlightDynamicsModel.JSBSimMovementComponent|SetCommands _jsbsimmovement (Utilities|Struct|MakeFlightControlCommands 0.0 0.0))))
  (:Released
    (Variables|Default|SetPressing%20W false)))

(event Input|KeyboardEvents|Tab
  (params (Key :type Key%20Structure))
  ;[0.15 0.15 0.15 0.5] Camera
  (:Pressed
    (Utilities|FlowControl|FlipFlop
      (:A
        (Components|Activation|SetActive (Variables|Default|GetTPCam) false false)
        (Components|Activation|SetActive (Variables|Default|GetCockpitCam) true false))
      (:B
        (Components|Activation|SetActive (Variables|Default|GetTPCam) true false)
        (Components|Activation|SetActive (Variables|Default|GetCockpitCam) false false)))))

(event Input|KeyboardEvents|S
  (params (Key :type Key%20Structure))
  (bind _jsbsimmovement (Variables|Default|GetJSBSimMovement))
  (bind _enginecommands (Variables|/Script/JSBSimFlightDynamicsModel.JSBSimMovementComponent|GetEngineCommands _jsbsimmovement))
  ;[1 1 1] 조종
  (:Pressed
    (Variables|Default|SetPressing%20S true)
    (for (_ _array_index) _enginecommands
      (Utilities|Struct|SetmembersinEngineCommand (Utilities|Array|Get(acopy) _enginecommands _array_index) (Variables|Default|GetThrottleValue))))
  (:Released
    (Variables|Default|SetPressing%20S false)))

(event Input|KeyboardEvents|A
  (params (Key :type Key%20Structure))
  ;[1 1 1] 조종
  (:Pressed
    (Variables|Default|SetPressing%20A true)
    (Variables|/Script/JSBSimFlightDynamicsModel.JSBSimMovementComponent|SetCommands (Variables|Default|GetJSBSimMovement) (Utilities|Struct|MakeFlightControlCommands (Variables|Default|GetRoll%20Trim))))
  (:Released
    (Variables|Default|SetPressing%20A false)))

(event Input|KeyboardEvents|D
  (params (Key :type Key%20Structure))
  ;[1 1 1] 조종
  (:Pressed
    (Variables|Default|SetPressing%20D true)
    (Variables|/Script/JSBSimFlightDynamicsModel.JSBSimMovementComponent|SetCommands (Variables|Default|GetJSBSimMovement) (Utilities|Struct|MakeFlightControlCommands (Variables|Default|GetRoll%20Trim))))
  (:Released
    (Variables|Default|SetPressing%20D false)))

(event Input|KeyboardEvents|E
  (params (Key :type Key%20Structure))
  ;[1 1 1] 조종
  (:Pressed
    (Variables|Default|SetPressing%20E true)
    (Variables|/Script/JSBSimFlightDynamicsModel.JSBSimMovementComponent|SetCommands (Variables|Default|GetJSBSimMovement) (Utilities|Struct|MakeFlightControlCommands (Variables|Default|GetPitch%20Trim))))
  (:Released
    (Variables|Default|SetPressing%20E false)))

(event Input|KeyboardEvents|C
  (params (Key :type Key%20Structure))
  ;[1 1 1] 조종
  (:Pressed
    (Variables|Default|SetPressing%20C true)
    (Variables|/Script/JSBSimFlightDynamicsModel.JSBSimMovementComponent|SetCommands (Variables|Default|GetJSBSimMovement) (Utilities|Struct|MakeFlightControlCommands (Variables|Default|GetPitch%20Trim))))
  (:Released
    (Variables|Default|SetPressing%20C false)))

(fn ConstructionScript)