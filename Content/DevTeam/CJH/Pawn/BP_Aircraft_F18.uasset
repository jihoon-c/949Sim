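; BP_Aircraft_F18 is an F-18 aircraft pawn that adds player input setup and camera control to its parent class.
; BeginPlay registers the IMC_Aircraft Enhanced Input mapping context on player 0.
; Legacy LookRight and LookUp axis events drive controller yaw and inverted pitch.
; A hardcoded Tab key uses a FlipFlop to swap between the third-person and cockpit cameras.
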(event EventBeginPlay
  ;[0.15 0.15 0.15 0.5] BeginPlay
  (|CallParentFunction)
  (Input|AddMappingContext (PlayerController|LocalPlayerSubsystems|GetEnhancedInputLocalPlayerSubsystem (Game|GetPlayerController 0)) "/Game/DevTeam/CJH/IA/IMC_Aircraft.IMC_Aircraft" 0 "(bIgnoreAllPressedKeysUntilRelease=True,bForceImmediately=False,bNotifyUserSettings=False)"))

(event EventTick
  (params (DeltaSeconds :type Float%20%28single-precision%29))
  ;[0.15 0.15 0.15 0.5] Tick
  (|CallParentFunction DeltaSeconds))

(event Input|AxisEvents|InputAxisLookUp
  (params (AxisValue :type Float%20%28single-precision%29))
  ;[0.15 0.15 0.15 0.5] Camera
  (Pawn|Input|AddControllerPitchInput (* AxisValue -1.0)))

(event Input|AxisEvents|InputAxisLookRight
  (params (AxisValue :type Float%20%28single-precision%29))
  ;[0.15 0.15 0.15 0.5] Camera
  (Pawn|Input|AddControllerYawInput AxisValue))

(event Input|KeyboardEvents|Tab
  (params (Key :type Key%20Structure :default "None"))
  ;[0.15 0.15 0.15 0.5] Camera
  (:Pressed
    (Utilities|FlowControl|FlipFlop
      (:A
        (Components|Activation|SetActive (Variables|Default|GetTPCam) false false)
        (Components|Activation|SetActive (Variables|Default|GetCockpitCam) true false))
      (:B
        (Components|Activation|SetActive (Variables|Default|GetTPCam) true false)
        (Components|Activation|SetActive (Variables|Default|GetCockpitCam) false false)))))

(fn ConstructionScript)